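; Player controller for kart races that handles local setup, race event relay, checkpoint reset and the pause menu.
; On BeginPlay the local controller clears widgets, copies PlayerInfo from the game instance and sets game-only input.
; On possess it binds the kart's checkpoint and finish events, forwarding them to the GameMode through RaceModesInterface.
; The menu key toggles a blurred pause overlay, while leaving or EndPlay destroys the online session.
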(event `self.ReceiveBeginPlay`
  ;[1 1 1] Event Begin Play - Entry Event
  (if (`self.IsLocalPlayerController`)
    (`WidgetLayoutLibrary.RemoveAllWidgets`)
    (`self.Load Game`)
    (`WidgetBlueprintLibrary.SetInputMode_GameOnly` self)))

(event `self.ReceivePossess`
  (params (PossessedPawn :type "Pawn Object Reference"))
  ;[1 1 1] On Possess - Bind Kart Events
  (bind _askart (cast `Kart` PossessedPawn))
  (add `Kart.OnCheckpointPassed` _askart (delegate `OnCheckpointPassed`))
  (add `Kart.OnRaceFinished` _askart (delegate `OnRaceFinished`)))

(event `OnRaceFinished`
  (params (FinishingPlayer :type "KartPlayerState Object Reference") (FinishingTime :type "Float (double-precision)"))
  (bind _returnvalue (`GameplayStatics.GetGameMode`))
  ;[1 1 1] On Possess - Bind Kart Events
  ;;[1 1 1] Race Finished
  (if (`KismetSystemLibrary.DoesImplementInterface` _returnvalue "/Script/AllanKart.RaceModesInterface")
    (message `RaceModesInterface.FinishedRace` _returnvalue FinishingPlayer FinishingTime)))

(event `OnCheckpointPassed`
  (params (Player :type "KartPlayerState Object Reference") (Lap :type Integer) (CheckpointNumber :type Integer) (RaceTime :type "Float (double-precision)"))
  (bind _returnvalue (`GameplayStatics.GetGameMode`))
  ;[1 1 1] On Possess - Bind Kart Events
  ;;[1 1 1] Pass Checkpoint
  (if (`KismetSystemLibrary.DoesImplementInterface` _returnvalue "/Script/AllanKart.RaceModesInterface")
    (message `RaceModesInterface.PassedCheckpoint` _returnvalue Player)))

(event `Key|NumPadZero`
  (params (Key :type "Key Structure"))
  ;[1 1 1] Reset to last checkpoint
  (:`Pressed`
    (`self.ResetToLastCheckpoint`)))

(event `InputAction|Editor_Menu`
  (params (Key :type "Key Structure"))
  ;[1 1 1] Pause Menu Setup
  (:`Pressed`
    (if (`self.IsPauseMenuUp`)
      (`self.Hide Pause Menu`)
      (else
        (`self.Show Pause Menu`)))))

(event `Show Pause Menu`
  (bind _blurry_background (`self.Blurry Background`))
  ;[1 1 1] Pause Menu Setup
  ;;[1 1 1] Show Pause Menu
  (`/Engine/EditorBlueprintResources/StandardMacros.IsValid` _blurry_background
    (:`Is Valid`
      (if (not (`Widget.IsInViewport` _blurry_background))
        (bind _returnvalue (`|CreateWidget` "/Game/SimpleMenuUI/UI/Widgets/GameplayWidgets/Widget_BlurryBackground.Widget_BlurryBackground_C" :!label _label))
        (bind _output_get (set `self.Blurry Background` _returnvalue))
        (`UserWidget.AddToViewport` _output_get 0)))
    (:`Is Not Valid`
      (goto _label)))
  (bind _returnvalue_2 (`|CreateWidget` "/Game/SimpleMenuUI/UI/Widgets/GameplayWidgets/Widget_PauseMenu.Widget_PauseMenu_C" self))
  (bind _output_get_2 (set `self.Pause Menu` _returnvalue_2))
  (`UserWidget.AddToViewport` _output_get_2 0)
  (`WidgetBlueprintLibrary.SetInputMode_GameAndUIEx` self _output_get_2)
  (set `self.bShowMouseCursor` true)
  (set `self.IsPauseMenuUp` true))

(event `Hide Pause Menu`
  ;[1 1 1] Pause Menu Setup
  ;;[1 1 1] Hide Pause Menu
  (`Widget.RemoveFromParent` (`self.Pause Menu`))
  (`Widget.RemoveFromParent` (`self.Blurry Background`))
  (bind _output_get (set `self.IsPauseMenuUp` false))
  (set `self.bShowMouseCursor` _output_get)
  (`WidgetBlueprintLibrary.SetInputMode_GameOnly` self))

(event `self.ReceiveEndPlay`
  (params (EndPlayReason :type "EEndPlayReason Enum" :default "Destroyed"))
  ;[1 1 1] Leave Session - End Play
  (`DestroySessionCallbackProxy.DestroySession` self :!label _label_2))

(event `Leave Session`
  ;[1 1 1] Leave Session - End Play
  (`GameplayStatics.OpenLevel` "Level_MainMenu")
  (goto _label_2))

(fn `Load Game`
  (bind _asblueprint_game_instance (cast `/Game/SimpleMenuUI/Blueprints/Global/Blueprint_GameInstance` (`GameplayStatics.GetGameInstance`)))
  (set `self.Player Info` (`/Game/SimpleMenuUI/Blueprints/Global/Blueprint_GameInstance.PlayerInfo` _asblueprint_game_instance)))

(fn `UserConstructionScript`)